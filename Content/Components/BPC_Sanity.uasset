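; Sanity component that tracks its owner's sanity as a clamped integer, with functions to raise and lower it.
; Decreases fire decreased and depleted events and trigger an effect check that picks a random row from tiered High, Medium or Low sanity data tables.
; Only the low tier, below 25, applies anything, adding the row's effect component to the owner; high and medium results go unused.
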(fn `DecreaseSanity`
  (params (Amount :type Integer))
  (bind _output_get (set `self.CurrentSanity` (`KismetMathLibrary.Clamp` (- (`self.CurrentSanity`) Amount) 0 (`self.MaxSanity`))))
  (`self.OnSanityDecreased`)
  (`self.TriggerSanityEffect`)
  (if (<= _output_get 0)
    (`self.OnSanityDepleted`))
  (return))

(fn `IncreaseSanity`
  (params (Amount :type Integer))
  (bind _output_get (set `self.CurrentSanity` (`KismetMathLibrary.Clamp` (+ (`self.CurrentSanity`) Amount) 0 (`self.MaxSanity`))))
  (if (>= _output_get 100)
    (`KismetSystemLibrary.PrintString` "Max Sanity"))
  (return))

(fn `TriggerSanityEffect`
  (bind _currentsanity (`self.CurrentSanity`))
  (bind _mediumsanity (`self.MediumSanity`))
  (bind _highsanity (`self.HighSanity`))
  (bind _lowsanity (`self.LowSanity`))
  (if (>= (`self.CurrentSanity`) 70)
    (bind _outrownames (`DataTableFunctionLibrary.GetDataTableRowNames` _highsanity))
    (bind _returnvalue (`|GetDataTableRow` _highsanity (`KismetArrayLibrary.Array_Random` _outrownames)))
    (elif (and (< _currentsanity 50) (> _currentsanity 25))
      (bind _outrownames_2 (`DataTableFunctionLibrary.GetDataTableRowNames` _mediumsanity))
      (bind _returnvalue_2 (`|GetDataTableRow` _mediumsanity (`KismetArrayLibrary.Array_Random` _outrownames_2)))
      (elif (< (`self.CurrentSanity`) 25)
        (bind _outrownames_3 (`DataTableFunctionLibrary.GetDataTableRowNames` _lowsanity))
        (bind _returnvalue_3 (`|GetDataTableRow` _lowsanity (`KismetArrayLibrary.Array_Random` _outrownames_3))
          (:`then`
            (`|AddComponentByClass` (`self.GetOwner`) (`.EffectComponent_8_37795BCB4D71CF5B9F798C83AE28DF87` (break `/Game/FirstPerson/Blueprints/DataTables/S_Sanity` _returnvalue_3)))))))))