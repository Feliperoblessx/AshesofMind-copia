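; BPC_Interaction is an actor component on the first-person character that detects interactable actors in view and shows an interaction prompt.
; Each tick it hides the prompt, then sphere-traces along the camera's forward vector, ignoring the held item, and stores the hit actor for GetInteractable.
; Non-BP_BaseItem hits implementing BPI_Interactable show the WBP_Interaction widget unless suppressed.
; Those checks also update the character's active-interactable flag and throw prompt visibility.
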(event `SetInteractionSuppressed`
  (params (Suppressed :type Boolean))
  (bind _wbp (`self.WBP`))
  (set `self.bInteractionSuppressed` Suppressed)
  (if (`self.bInteractionSuppressed`)
    (`Widget.SetVisibility` _wbp "Collapsed")
    (else
      (`Widget.SetVisibility` _wbp "Visible"))))

(event `self.ReceiveTick`
  (params (DeltaSeconds :type "Float (single-precision)"))
  (bind _returnvalue (`self.GetOwner`))
  (bind _wbp (`self.WBP`))
  (bind _wbp_2 (`self.WBP`))
  (bind _returnvalue_2 (`Actor.K2_GetActorLocation` (`self.GetOwner`)))
  (`|ExecutionSequence`
    (:`then_0`
      (`Widget.RemoveFromParent` _wbp_2)
      (`Widget.SetVisibility` _wbp_2 "Collapsed"))
    (:`then_1`
      ; Ignorar cuando ya tiene el objeto en la mano
      (bind _asbp_first_person_character (cast `/Game/FirstPerson/Blueprints/BP_FirstPersonCharacter` (`self.GetOwner`)))
      (bind _outhit (`KismetSystemLibrary.SphereTraceSingle` (+ _returnvalue_2 (0.0 0.0 50.0)) (+ _returnvalue_2 (* (`Actor.GetActorForwardVector` (`GameplayStatics.GetPlayerCameraManager` 0)) 400.0) (0.0 0.0 50.0)) 25.0 "TraceTypeQuery1" false (`|MakeArray` (`/Game/FirstPerson/Blueprints/BP_FirstPersonCharacter.PickUpItem` _asbp_first_person_character))))
      (if true
        (bind (_bblockinghit _binitialoverlap _time _distance _location _impactpoint _normal _impactnormal _physmat _hitactor) (`GameplayStatics.BreakHitResult` _outhit))
        (bind _output_get (set `self.Active Interactable` _hitactor))
        (cast `/Game/FirstPerson/Blueprints/Interactables/Fragementos_Items_Lore/BP_BaseItem` _hitactor
          (:`then`
            (`Widget.SetVisibility` (`self.WBP`) "Hidden"))
          (:`CastFailed`
            (`self.IsInteractable` _output_get
              (:`true`
                (bind _asbp_first_person_character_2 (cast `/Game/FirstPerson/Blueprints/BP_FirstPersonCharacter` _returnvalue))
                (set `/Game/FirstPerson/Blueprints/BP_FirstPersonCharacter.Has Active Interactable` true _asbp_first_person_character_2)
                (`/Game/FirstPerson/Blueprints/BP_FirstPersonCharacter.Update Throw Prompt Visibility` _asbp_first_person_character_2)
                (if (not (`self.bInteractionSuppressed`))
                  (`UserWidget.AddToViewport` _wbp 0)
                  (`Widget.SetVisibility` _wbp "Visible")))
              (:`false`
                (bind _asbp_first_person_character_3 (cast `/Game/FirstPerson/Blueprints/BP_FirstPersonCharacter` _returnvalue :!label _label))
                (set `/Game/FirstPerson/Blueprints/BP_FirstPersonCharacter.Has Active Interactable` false _asbp_first_person_character_3)
                (`/Game/FirstPerson/Blueprints/BP_FirstPersonCharacter.Update Throw Prompt Visibility` _asbp_first_person_character_3)))))
        (else
          (set `self.Active Interactable` null)
          (goto _label))))))

(event `self.ReceiveBeginPlay`
  (bind _returnvalue (`|CreateWidget` "/Game/Widgets/WBP_Interaction.WBP_Interaction_C"))
  (set `self.WBP` _returnvalue))

(fn `GetInteractable`
  (returns (Interactable :type "Actor Object Reference"))
  (return (`self.Active Interactable`)))